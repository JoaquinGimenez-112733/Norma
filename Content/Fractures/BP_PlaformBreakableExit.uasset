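; Breakable exit platform that triggers what appears to be the game's exit screen when it fractures.
; The Geometry Collection's Chaos break event passes through a DoOnce, so only the first break counts.
; That break adds the WBP_GGExit widget to the viewport and switches player 0's view target to this actor using an ease-out blend function.
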(event `self.GeometryCollectionComponent.OnChaosBreakEvent`
  (params (BreakEvent :type "ChaosBreakEvent Structure (by ref)"))
  (`/Engine/EditorBlueprintResources/StandardMacros.DoOnce` false
    (:`Completed`
      (bind _returnvalue (`|CreateWidget` "/Game/UI/WBP_GGExit.WBP_GGExit_C"))
      (`UserWidget.AddToViewport` _returnvalue 1)
      (`PlayerController.SetViewTargetWithBlend` (`GameplayStatics.GetPlayerController` 0) self 0.0 "VTBlend_EaseOut" 1.0 false))))

(fn `UserConstructionScript`
  (`parent.UserConstructionScript`))