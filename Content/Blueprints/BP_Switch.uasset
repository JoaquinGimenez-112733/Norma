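; BP_Switch is a switch that moves a referenced platform, OMovingPlatform3, when BP_Norma enters its box.
; The overlap only acts once the Interact input has set Interacted, which is never reset.
; It prints a debug message and calls MovePlatform with one of two opposite X targets chosen by Switch.
; Switch is then ANDed with false, so it always ends false rather than toggling.
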(event `self.Box.OnComponentBeginOverlap`
  (params (OverlappedComponent :type "PrimitiveComponent Object Reference") (OtherActor :type "Actor Object Reference") (OtherComp :type "PrimitiveComponent Object Reference") (OtherBodyIndex :type Integer) (bFromSweep :type Boolean) (SweepResult :type "HitResult Structure (by ref)"))
  (cast `/Game/Blueprints/Norma/BP_Norma` OtherActor)
  (if (stale `InputAction|DeprecatedInteract` _output_get)
    (`KismetSystemLibrary.PrintString` "Hello")
    (if (`self.bSwitch`)
      (set `self.TargetPosition` (-4000.0 0.0 0.0))
      (else
        (set `self.TargetPosition` (4000.0 0.0 0.0))))
    (`/Game/Blueprints/Platforms/BP_MovingPlatformChild3.MovePlatform` (`self.oMovingPlatform3`) (`self.TargetPosition`))
    (set `self.bSwitch` (and (`self.bSwitch`) false))))

(event `InputAction|DeprecatedInteract`
  (params (Key :type "Key Structure"))
  (:`Pressed`
    (bind _output_get (set `self.bInteracted` true))))

(fn `UserConstructionScript`)