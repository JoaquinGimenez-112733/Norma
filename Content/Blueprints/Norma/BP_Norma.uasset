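; Norma, the player character: a side-scrolling runner and jumper with coyote time, crouch, interaction, and a bounce that breaks destructible geometry on fast falls.
; A looping timer drains her light, driving point light intensity and four segmented HUD bars.
; At zero, a delayed timer removes a bar and lowers maximum light; consuming a "Bichito de luz" refills light and cancels that timer.
; Coyote time combines a retriggerable delay with a CanJumpInternal override.
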(event `/Game/Blueprints/Interfaces/BPI_Consume.ConsumeBichitoDeLuz`
  ;[1 1 1] Consume Bichito de luz Section
  (set `self.ActualLighting` (`KismetMathLibrary.FClamp` (+ 100000.0 (`self.ActualLighting`)) 0.0 (`self.MaxLighting`)))
  (`KismetSystemLibrary.K2_ClearAndInvalidateTimerHandle` (`self.HandleLightD`)))

(event `InputAction|DeprecatedInteract`
  (params (Key :type "Key Structure"))
  ;[1 1 1] Interact Section
  (:`Pressed`
    (for _array_element (`self.GetOverlappingActors` "/Script/Engine.Actor")
      (if (`KismetSystemLibrary.DoesImplementInterface` _array_element "/Game/Blueprints/Interfaces/BI_Interact.BI_Interact_C")
        (message `/Game/Blueprints/Interfaces/BI_Interact.Interact` _array_element)
        (break)))))

(event `self.ReceiveBeginPlay`
  (bind _listbars (`self.ListBars`))
  ;[0 0.2393 1] BEGIN PLAY
  (`self.Implement Mapping Context`)
  (bind _returnvalue (`|CreateWidget` "/Game/UI/WBP_ProgressLight.WBP_ProgressLight_C"))
  (bind _output_get (set `self.PB_Widget` _returnvalue))
  (`UserWidget.AddToViewport` _output_get 0)
  (bind _pb_000_050 (`/Game/UI/WBP_ProgressLight.PB_000_050` _output_get))
  (set `self.PB 000 050` _pb_000_050)
  (bind _pb_050_100 (`/Game/UI/WBP_ProgressLight.PB_050_100` _output_get))
  (set `self.PB 050 100` _pb_050_100)
  (bind _pb_100_150 (`/Game/UI/WBP_ProgressLight.PB_100_150` _output_get))
  (set `self.PB 100 150` _pb_100_150)
  (bind _pb_150_200 (`/Game/UI/WBP_ProgressLight.PB_150_200` _output_get))
  (set `self.PB 150 200` _pb_150_200)
  (`KismetArrayLibrary.Array_Add` (`self.ListBars`) _pb_000_050)
  (`KismetArrayLibrary.Array_Add` (`self.ListBars`) _pb_050_100)
  (`KismetArrayLibrary.Array_Add` (`self.ListBars`) _pb_100_150)
  (`KismetArrayLibrary.Array_Add` _listbars _pb_150_200)
  (bind _output_get_2 (set `self.MaxLighting` (`KismetMathLibrary.Conv_IntToDouble` (* (`KismetArrayLibrary.Array_Length` _listbars) 50))))
  (set `self.ActualLighting` _output_get_2)
  (`KismetSystemLibrary.K2_SetTimerDelegate` (delegate `LightD`) 0.25 true true))

(event `self.ReceiveTick`
  (params (DeltaSeconds :type "Float (single-precision)"))
  ;[1 0 0] TICK
)

(event `LightD`
  (bind _returnvalue (`KismetMathLibrary.FClamp` (+ (`self.ActualLighting`) (`self.LightingDecay`)) 0.0 250.0))
  ;[0 0.2393 1] BEGIN PLAY
  (bind _output_get (set `self.ActualLighting` _returnvalue))
  (`self.SetPercentsPB` _output_get)
  (`LightComponent.SetIntensity` (`self.PointLight`) _output_get)
  (if (== _returnvalue 0.0)
    (if (not (`KismetSystemLibrary.K2_IsTimerActiveHandle` (`self.HandleLightD`)))
      (bind _returnvalue_2 (`KismetSystemLibrary.K2_SetTimerDelegate` (delegate `HurryUpLighD`) 5.0))
      (set `self.HandleLightD` _returnvalue_2))))

(event `HurryUpLighD`
  ;[0 0.2393 1] BEGIN PLAY
  (`self.Hide`))

(event `EnhancedInput|/Game/Input/Actions/IA_NormaMove`
  (params (ActionValue :type "Float (double-precision)") (ElapsedSeconds :type "Float (double-precision)") (TriggeredSeconds :type "Float (double-precision)") (InputAction :type "InputAction Object Reference" :default "/Game/Input/Actions/IA_NormaMove.IA_NormaMove"))
  ;[1 1 1] Movement and rotation section
  (:`Triggered`
    (`self.FUNC_Movement` ActionValue ActionValue)))

(event `EnhancedInput|/Game/Input/Actions/IA_Restart`
  (params (ActionValue :type Boolean) (ElapsedSeconds :type "Float (double-precision)") (TriggeredSeconds :type "Float (double-precision)") (InputAction :type "InputAction Object Reference" :default "/Game/Input/Actions/IA_Restart.IA_Restart"))
  ;[1 1 1] Restart Level
  (:`Triggered`
    (`KismetSystemLibrary.ExecuteConsoleCommand` "RestartLevel" null)))

(event `EnhancedInput|/Game/Input/Actions/IA_NormaJump`
  (params (ActionValue :type Boolean) (ElapsedSeconds :type "Float (double-precision)") (TriggeredSeconds :type "Float (double-precision)") (InputAction :type "InputAction Object Reference" :default "/Game/Input/Actions/IA_NormaJump.IA_NormaJump"))
  ;[1 1 1] JUMP SECTION
  (:`Started`
    (`self.UnCrouch`)
    (`KismetSystemLibrary.Delay` 0.001)
    (set `self.JumpDown` true)
    (`self.Jump`))
  (:`Completed`
    (set `self.JumpDown` false)
    (`self.StopJumping`)))

(event `InputAction|DeprecatedCrouching`
  (params (Key :type "Key Structure"))
  ;[1 1 1] Crouch Section
  (:`Pressed`
    (`self.Crouch`))
  (:`Released`
    (`self.UnCrouch`)))

(event `self.OnJumped`
  (`PaperZDAnimInstance.JumpToNode` (`PaperZDAnimationComponent.AnimInstance` (`self.AnimationComponent`)) "Airborne" "None"))

(event `EnhancedInput|/Game/Input/Actions/IA_CloseGame`
  (params (ActionValue :type Boolean) (ElapsedSeconds :type "Float (double-precision)") (TriggeredSeconds :type "Float (double-precision)") (InputAction :type "InputAction Object Reference" :default "/Game/Input/Actions/IA_CloseGame.IA_CloseGame"))
  (:`Triggered`
    (`KismetSystemLibrary.QuitGame` null "Quit")))

(event `self.OnWalkingOffLedge`
  (params (PreviousFloorImpactNormal :type "Vector Structure (by ref)") (PreviousFloorContactNormal :type "Vector Structure (by ref)") (PreviousLocation :type "Vector Structure (by ref)") (TimeDelta :type "Float (single-precision)"))
  ;[0.9739 1 0.0772] on Jumped or off Ledge - Airborne
  (`PaperZDAnimInstance.JumpToNode` (`PaperZDAnimationComponent.AnimInstance` (`self.AnimationComponent`)) "Airborne" "None")
  (set `self.bCoyoteable` true)
  (`KismetSystemLibrary.RetriggerableDelay` 0.15)
  (set `self.bCoyoteable` false))

(event `self.FootCollider.OnComponentBeginOverlap`
  (params (OverlappedComponent :type "PrimitiveComponent Object Reference") (OtherActor :type "Actor Object Reference") (OtherComp :type "PrimitiveComponent Object Reference") (OtherBodyIndex :type Integer) (bFromSweep :type Boolean) (SweepResult :type "HitResult Structure (by ref)"))
  (bind (_returnvalue_x _returnvalue_y _returnvalue_z) (`KismetMathLibrary.BreakVector` (`CharacterMovementComponent.GetLastUpdateVelocity` (`self.CharacterMovement`))))
  (bind _asgeometry_collection_actor (cast `GeometryCollectionActor` OtherActor))
  (if (< _returnvalue_z -3000.0)
    (bind _returnvalue (`|SpawnActorFromClass` "/Game/Blueprints/BP_Damage.BP_Damage_C" (`KismetMathLibrary.Conv_VectorToTransform` (`self.K2_GetActorLocation` _asgeometry_collection_actor)) "Undefined" "MultiplyWithRoot" null null))
    (`KismetSystemLibrary.Delay` 0.01)
    (`self.K2_DestroyActor` _returnvalue)
    (`self.LaunchCharacter` (0.0 0.0 1200.0))
    (bind _returnvalue_2 (`GameplayStatics.SpawnSoundAtLocation` "/Game/Sound/SFX/GlassBreaking/SC_GlassBreaking.SC_GlassBreaking" (0.0 0.0 0.0) (struct) 1.0 1.0 0.0 null null))
    (`AudioComponent.Play` _returnvalue_2 0.0)))

(fn `CanJumpInternal`
  (returns (ReturnValue :type Boolean))
  (bind _returnvalue (`parent.CanJumpInternal`))
  (return (or _returnvalue (`self.bCoyoteable`))))

(fn `FUNC Light Decay`
  (params (A :type "Float (double-precision)"))
  (bind _returnvalue (`KismetMathLibrary.FClamp` (+ (`self.ActualLighting`) (* A (`self.LightingDecay`))) 0.0 250.0))
  (bind _output_get (set `self.ActualLighting` _returnvalue))
  (if (> _returnvalue 0.0)
    (`self.SetPercentsPB` _output_get)
    (`LightComponent.SetIntensity` (`self.PointLight`) _output_get)))

(fn `FUNC_Movement`
  (params (A :type "Float (double-precision)") (ScaleValue :type "Float (single-precision)"))
  (`self.AddMovementInput` (1.0 0.0 0.0) ScaleValue)
  (`Controller.SetControlRotation` (`self.GetController`) (select `bool` (> A 0.0) :`false` (`KismetMathLibrary.MakeRotator` 0.0 0.0 180.0) :`true` (`KismetMathLibrary.MakeRotator` 0.0))))

(fn `Hide`
  (bind _listbars (`self.ListBars`))
  (bind _output (`|GetArrayItem` _listbars (`KismetArrayLibrary.Array_LastIndex` _listbars)))
  (if (`KismetSystemLibrary.IsValid` _output)
    (`Widget.SetVisibility` _output "Collapsed")
    (`KismetArrayLibrary.Array_RemoveItem` _listbars _output)
    (set `self.MaxLighting` (`KismetMathLibrary.Conv_IntToDouble` (* (`KismetArrayLibrary.Array_Length` _listbars) 50)))))

(fn `Implement Mapping Context`
  (bind _asplayer_controller (cast `PlayerController` (`self.GetController`)))
  (`EnhancedInputSubsystemInterface.AddMappingContext` (pcsubsystem `EnhancedInputLocalPlayerSubsystem` _asplayer_controller) "/Game/Input/IMC_Norma.IMC_Norma" 0 (struct)))

(fn `SetPercentsPB`
  (params (ActualLight :type "Float (double-precision)"))
  (`|ExecutionSequence`
    (:`then_0`
      (`ProgressBar.SetPercent` (`self.PB 000 050`) (`KismetMathLibrary.FClamp` (/ (- ActualLight 0.0) 50.0))))
    (:`then_1`
      (`ProgressBar.SetPercent` (`self.PB 050 100`) (`KismetMathLibrary.FClamp` (/ (- ActualLight 50.0) 50.0))))
    (:`then_2`
      (`ProgressBar.SetPercent` (`self.PB 100 150`) (`KismetMathLibrary.FClamp` (/ (- ActualLight 100.0) 50.0))))
    (:`then_3`
      (`ProgressBar.SetPercent` (`self.PB 150 200`) (`KismetMathLibrary.FClamp` (/ (- ActualLight 150.0) 50.0))))))

(fn `UserConstructionScript`)