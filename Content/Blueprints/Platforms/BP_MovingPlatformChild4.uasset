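; Moving platform child Blueprint that slides along X at a fixed height and lets BP_Norma pass through it.
; MovePlatform1 toggles a Timeline between play and reverse, setting relative location with a mechanism sound.
; Overlapping Underneath, or Underneath1 while crouching, disables RenderComponent collision; only leaving Underneath restores it.
; InterpToMovement logic is left unconnected.
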(event `self.Underneath.OnComponentBeginOverlap`
  (params (OverlappedComponent :type "PrimitiveComponent Object Reference") (OtherActor :type "Actor Object Reference") (OtherComp :type "PrimitiveComponent Object Reference") (OtherBodyIndex :type Integer) (bFromSweep :type Boolean) (SweepResult :type "HitResult Structure (by ref)"))
  (cast `/Game/Blueprints/Norma/BP_Norma` OtherActor)
  (`PrimitiveComponent.SetCollisionEnabled` (`self.RenderComponent`) "NoCollision"))

(event `self.Underneath.OnComponentEndOverlap`
  (params (OverlappedComponent :type "PrimitiveComponent Object Reference") (OtherActor :type "Actor Object Reference") (OtherComp :type "PrimitiveComponent Object Reference") (OtherBodyIndex :type Integer))
  (cast `/Game/Blueprints/Norma/BP_Norma` OtherActor)
  (`PrimitiveComponent.SetCollisionEnabled` (`self.RenderComponent`) "QueryAndPhysics"))

(event `self.Underneath1.OnComponentBeginOverlap`
  (params (OverlappedComponent :type "PrimitiveComponent Object Reference") (OtherActor :type "Actor Object Reference") (OtherComp :type "PrimitiveComponent Object Reference") (OtherBodyIndex :type Integer) (bFromSweep :type Boolean) (SweepResult :type "HitResult Structure (by ref)"))
  (bind _asbp_norma (cast `/Game/Blueprints/Norma/BP_Norma` OtherActor))
  (if (`NavMovementComponent.IsCrouching` (`Character.CharacterMovement` _asbp_norma))
    (`PrimitiveComponent.SetCollisionEnabled` (`self.RenderComponent`) "NoCollision")))

(event `self.Underneath1.OnComponentEndOverlap`
  (params (OverlappedComponent :type "PrimitiveComponent Object Reference") (OtherActor :type "Actor Object Reference") (OtherComp :type "PrimitiveComponent Object Reference") (OtherBodyIndex :type Integer))
  (cast `/Game/Blueprints/Norma/BP_Norma` OtherActor))

(event `self.ReceiveBeginPlay`)

(event `self.MovePlatform1`
  (`AudioComponent.Play` (`self.MechanismSound`) 0.0)
  (if (`self.Moved`)
    (set `self.Moved` false)
    (bind (_direction _newtrack_0) (`Timeline|Timeline` :!via `Reverse` :!label _label)
      (:`Update`
        (set `self.Target` _newtrack_0)
        (`self.Move Platform` (`self.Target`)))
      (:`Finished`
        (`AudioComponent.Stop` (`self.MechanismSound`))))
    (else
      (set `self.Moved` true)
      (goto _label))))

(fn `Move Platform`
  (params (TargetPosition :type "Vector Structure"))
  (locals (NewLocalVar :type "InterpControlPoint Structure"))
  (`self.K2_SetActorRelativeLocation` (`KismetMathLibrary.MakeVector` TargetPosition_X 0.0 -4540.0)))

(fn `UserConstructionScript`
  (`parent.UserConstructionScript`))