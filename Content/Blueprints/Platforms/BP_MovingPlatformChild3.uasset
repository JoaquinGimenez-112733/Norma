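; BP_MovingPlatformChild3 is a child moving platform Blueprint driven by an InterpToMovement component.
; BeginPlay stores the actor's starting location.
; MovePlatform prints a debug string, writes the target as a relative control point at index 1 of ControlPoints, then activates the component without reset.
; The node assigning ControlPoints to InterpToMovement is unconnected, so that explicit assignment never runs.
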(event `self.ReceiveBeginPlay`
  (set `self.StartLocation` (`self.K2_GetActorLocation`)))

(fn `MovePlatform`
  (params (TargetPosition :type "Vector Structure"))
  (`KismetSystemLibrary.PrintString` "funca")
  (`KismetArrayLibrary.Array_Set` (`self.Control Points`) 1 (make `InterpControlPoint` (`local.TargetPosition`)))
  (`ActorComponent.Activate` (`self.InterpToMovement`) false))

(fn `UserConstructionScript`
  (`parent.UserConstructionScript`))