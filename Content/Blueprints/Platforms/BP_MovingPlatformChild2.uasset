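; Moving platform child that toggles its collision so BP_Norma can pass through it, keeping the parent's tick.
; Overlapping the Underneath volume disables RenderComponent collision, and leaving restores it.
; Entering Underneath1 while crouching also disables collision, as does deprecated crouch input once FlagTop is set by Underneath.
; An IA_Crouch gate also leads to disabling collision, but its open and close logic is unwired.
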(event `self.ReceiveTick`
  (params (DeltaSeconds :type "Float (single-precision)"))
  (`parent.ReceiveTick` DeltaSeconds))

(event `self.Underneath.OnComponentBeginOverlap`
  (params (OverlappedComponent :type "PrimitiveComponent Object Reference") (OtherActor :type "Actor Object Reference") (OtherComp :type "PrimitiveComponent Object Reference") (OtherBodyIndex :type Integer) (bFromSweep :type Boolean) (SweepResult :type "HitResult Structure (by ref)"))
  (cast `/Game/Blueprints/Norma/BP_Norma` OtherActor)
  (`PrimitiveComponent.SetCollisionEnabled` (`self.RenderComponent`) "NoCollision")
  (set `self.Flag_Top` true))

(event `InputAction|DeprecatedCrouching`
  (params (Key :type "Key Structure"))
  (bind _returnvalue (`GameplayStatics.GetPlayerController` 0))
  (:`Pressed`
    (`self.EnableInput` _returnvalue)
    (set `self.Flag_Crouching` true)
    (if (and (`self.Flag_Top`) (`self.Flag_Crouching`)) :!label _label
      (`PrimitiveComponent.SetCollisionEnabled` (`self.RenderComponent`) "NoCollision")))
  (:`Released`
    (`self.DisableInput` _returnvalue)
    (set `self.Flag_Crouching` false)
    (goto _label)))

(event `self.Underneath.OnComponentEndOverlap`
  (params (OverlappedComponent :type "PrimitiveComponent Object Reference") (OtherActor :type "Actor Object Reference") (OtherComp :type "PrimitiveComponent Object Reference") (OtherBodyIndex :type Integer))
  (cast `/Game/Blueprints/Norma/BP_Norma` OtherActor)
  (`PrimitiveComponent.SetCollisionEnabled` (`self.RenderComponent`) "QueryAndPhysics")
  (set `self.Flag_Down` true))

(event `self.Underneath1.OnComponentBeginOverlap`
  (params (OverlappedComponent :type "PrimitiveComponent Object Reference") (OtherActor :type "Actor Object Reference") (OtherComp :type "PrimitiveComponent Object Reference") (OtherBodyIndex :type Integer) (bFromSweep :type Boolean) (SweepResult :type "HitResult Structure (by ref)"))
  (bind _asbp_norma (cast `/Game/Blueprints/Norma/BP_Norma` OtherActor))
  (if (`NavMovementComponent.IsCrouching` (`Character.CharacterMovement` _asbp_norma))
    (`PrimitiveComponent.SetCollisionEnabled` (`self.RenderComponent`) "NoCollision")))

(event `EnhancedInput|/Game/Input/Actions/IA_Crouch`
  (params (ActionValue :type Boolean) (ElapsedSeconds :type "Float (double-precision)") (TriggeredSeconds :type "Float (double-precision)") (InputAction :type "InputAction Object Reference" :default "/Game/Input/Actions/IA_Crouch.IA_Crouch"))
  (:`Triggered`
    (`/Engine/EditorBlueprintResources/StandardMacros.Gate` true
      (:`Exit`
        (`PrimitiveComponent.SetCollisionEnabled` (`self.RenderComponent`) "NoCollision")))))

(event `self.Underneath1.OnComponentEndOverlap`
  (params (OverlappedComponent :type "PrimitiveComponent Object Reference") (OtherActor :type "Actor Object Reference") (OtherComp :type "PrimitiveComponent Object Reference") (OtherBodyIndex :type Integer))
  (cast `/Game/Blueprints/Norma/BP_Norma` OtherActor))

(fn `UserConstructionScript`
  (`parent.UserConstructionScript`))