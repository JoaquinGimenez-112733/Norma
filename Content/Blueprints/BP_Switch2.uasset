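; BP_Switch2 is an interactable sprite-based lever switch that controls a moving platform.
; Each Interact messages the first BP_MovingPlatformChild4 found at BeginPlay, then toggles Switch to play or reverse a timeline that pitches the Rod.
; Box overlap, currently unfiltered though intended only for Norma, swaps Base and Rod to dynamic outline materials with timeline-animated Thickness; ending overlap restores the translucent lit sprite material.
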(event `self.Interact`
  (message `/Game/Blueprints/Interfaces/BI_MovePlatform1.MovePlatform1` (`self.oMovingPlatform4`))
  (if (`self.bSwitch`)
    (set `self.bSwitch` false)
    (bind (_direction _newtrack_1) (`Timeline|Timeline` :!via `Reverse` :!label _label)
      (:`Update`
        (`SceneComponent.K2_SetRelativeRotation` (`self.Rod`) (`KismetMathLibrary.MakeRotator` 0.0 _newtrack_1) false false)))
    (else
      (set `self.bSwitch` true)
      (goto _label))))

(event `self.ReceiveBeginPlay`
  (bind _outactors (`GameplayStatics.GetAllActorsOfClass` "/Game/Blueprints/Platforms/BP_MovingPlatformChild4.BP_MovingPlatformChild4_C"))
  (set `self.oMovingPlatform4` (`|GetArrayItem` _outactors))
  (bind _returnvalue (`KismetMaterialLibrary.CreateDynamicMaterialInstance` "/Game/Materials/M_OutlineSprite.M_OutlineSprite"))
  (set `self.MID_OutlineBase` _returnvalue)
  (bind _returnvalue_2 (`KismetMaterialLibrary.CreateDynamicMaterialInstance` "/Game/Materials/M_OutlineRod.M_OutlineRod"))
  (set `self.MID_OutlineRod` _returnvalue_2))

(event `self.Box.OnComponentBeginOverlap`
  (params (OverlappedComponent :type "PrimitiveComponent Object Reference") (OtherActor :type "Actor Object Reference") (OtherComp :type "PrimitiveComponent Object Reference") (OtherBodyIndex :type Integer) (bFromSweep :type Boolean) (SweepResult :type "HitResult Structure (by ref)"))
  ;[1 1 1] Acá se anima el outline del switch al overlapear con ALGO (debería ser solo Norma)
  (`PrimitiveComponent.SetMaterial` (`self.Base`) 0 (`self.MID_OutlineBase`))
  (`PrimitiveComponent.SetMaterial` (`self.Rod`) 0 (`self.MID_OutlineRod`))
  (bind (_direction _newtrack_0) (`Timeline|Timeline_0` :!via `PlayFromStart`)
    (:`Update`
      (`MaterialInstanceDynamic.SetScalarParameterValue` (`self.MID_OutlineBase`) "Thickness" _newtrack_0)
      (`MaterialInstanceDynamic.SetScalarParameterValue` (`self.MID_OutlineRod`) "Thickness" _newtrack_0))))

(event `self.Box.OnComponentEndOverlap`
  (params (OverlappedComponent :type "PrimitiveComponent Object Reference") (OtherActor :type "Actor Object Reference") (OtherComp :type "PrimitiveComponent Object Reference") (OtherBodyIndex :type Integer))
  ;[1 1 1] Acá se anima el outline del switch al overlapear con ALGO (debería ser solo Norma)
  (`PrimitiveComponent.SetMaterial` (`self.Base`) 0 "/Paper2D/TranslucentLitSpriteMaterial.TranslucentLitSpriteMaterial")
  (`PrimitiveComponent.SetMaterial` (`self.Rod`) 0 "/Paper2D/TranslucentLitSpriteMaterial.TranslucentLitSpriteMaterial"))

(fn `UserConstructionScript`)